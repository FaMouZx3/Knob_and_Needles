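; MyCharacter is a character Blueprint that shows a health bar widget and keeps it facing the player's camera.
; Every tick it casts the widget component's user widget to HealthBar and sets the progress bar to Health divided by 100.
; It then rotates a scene component toward the player camera manager's location with a look-at rotation, creating a billboard effect.
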(event `self.ReceiveTick`
  (params (DeltaSeconds :type "Float (single-precision)"))
  (bind _scene (`self.Scene`))
  (bind _ashealth_bar (cast `/Game/Blueprint/UI_Blueprints/HealthBar` (`WidgetComponent.GetUserWidgetObject` (`self.Widget`))))
  (`ProgressBar.SetPercent` (`/Game/Blueprint/UI_Blueprints/HealthBar.ProgressBar_50` _ashealth_bar) (/ (`self.Health`) 100.0))
  (`SceneComponent.K2_SetWorldRotation` _scene (`KismetMathLibrary.FindLookAtRotation` (`SceneComponent.K2_GetComponentLocation` _scene) (`self.K2_GetActorLocation` (`GameplayStatics.GetPlayerCameraManager` 0))) false false))

(fn `UserConstructionScript`)