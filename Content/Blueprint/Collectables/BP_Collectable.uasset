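; BP_Collectable is a pickup, noted as a bomb, that attaches to the player character's left hand.
; Each Tick checks the Collision and IsSocketed flags, then calls OnPickedUp and finds the character through the PlayerReference's player ID.
; The static mesh snaps to the hand prop socket on MyCharacterBP, keeping world scale, and IsSocketed is set to prevent repeat attachment.
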(event `self.ReceiveTick`
  (params (DeltaSeconds :type "Float (single-precision)"))
  ;[1 1 1] Attach the Bomb on the Left Hand - Tom
  (if (`self.Collision`)
    (if (not (`self.IsSocketed`))
      (`self.OnPickedUp`)
      (bind _asmy_character_bp (cast `/Game/Blueprint/Character_BP/MyCharacterBP` (`GameplayStatics.GetPlayerCharacter` (`/Game/Blueprint/Character_BP/MyCharacterBP.MyPlayerID` (`self.PlayerReference`)))))
      (`SceneComponent.K2_AttachToComponent` (`self.StaticMesh`) (`/Game/Blueprint/Character_BP/MyCharacterBP.LeftHandProp_Socket` _asmy_character_bp) "hand_L_HoldProp_Socket" "SnapToTarget" "SnapToTarget" "KeepWorld" true)
      (set `self.IsSocketed` true))))

(fn `UserConstructionScript`)