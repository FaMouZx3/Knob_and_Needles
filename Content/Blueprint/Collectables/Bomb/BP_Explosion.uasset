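; Explosion actor for the bomb collectable, producing particles, a physics impulse, sound and an expanding shockwave.
; On BeginPlay it creates a dynamic material for the shockwave sphere, activates the particle system and starts a short timer.
; When the timer fires, it triggers the radial force and sound, then a timeline drives the sphere's scale and material opacity.
; The sphere component is destroyed when the timeline finishes, but the actor itself is not.
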(event `self.ReceiveBeginPlay`
  ;[1 1 1] create dynamic material-David
  (bind _returnvalue (`KismetMaterialLibrary.CreateDynamicMaterialInstance` (`PrimitiveComponent.GetMaterial` (`self.Sphere`) 0)))
  (bind _output_get (set `self.shockwave_Material` _returnvalue))
  (`PrimitiveComponent.SetMaterial` (`self.Sphere`) 0 _output_get)
  ;[1 1 1] Explosion - Tom / David
  (`ActorComponent.Activate` (`self.ParticleSystem`) false)
  (`KismetSystemLibrary.K2_SetTimerDelegate` (delegate `Particle Spawn`) 0.4))

(event `Particle Spawn`
  (bind _sphere (`self.Sphere`))
  ;[1 1 1] Explosion - Tom / David
  (`RadialForceComponent.FireImpulse` (`self.RadialForce`))
  (`GameplayStatics.PlaySoundAtLocation` "/Game/ScriptReferences/StarterContent/Audio/Explosion01.Explosion01" (`SceneComponent.K2_GetComponentLocation` (`self.DefaultSceneRoot`)))
  ;[1 1 1] Spawn material and scale animation-David
  (bind (_direction _expanse _opacity) (`Timeline|Timeline_0` :!via `PlayFromStart`)
    (:`Update`
      (`SceneComponent.SetWorldScale3D` _sphere (`KismetMathLibrary.Conv_DoubleToVector` _expanse))
      (`MaterialInstanceDynamic.SetScalarParameterValue` (`self.shockwave_Material`) "Opacity" _opacity))
    (:`Finished`
      (`ActorComponent.K2_DestroyComponent` _sphere))))

(fn `UserConstructionScript`)