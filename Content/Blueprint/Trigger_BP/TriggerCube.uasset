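; TriggerCube is a kill-volume trigger that handles respawning the player character after falling.
; On overlap with a MyCharacterBP, it teleports the character to its SpawnPoint, removes one life and sets HP back to 1.0.
; If no lives remain at the moment of overlap, it sets HP to zero and destroys the character instead.
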(event `self.TriggerCube.OnComponentBeginOverlap`
  (params (OverlappedComponent :type "PrimitiveComponent Object Reference") (OtherActor :type "Actor Object Reference") (OtherComp :type "PrimitiveComponent Object Reference") (OtherBodyIndex :type Integer) (bFromSweep :type Boolean) (SweepResult :type "HitResult Structure (by ref)"))
  ;[1 1 1] Respawn after falling - Tim
  (bind _asmy_character_bp (cast `/Game/Blueprint/Character_BP/MyCharacterBP` OtherActor))
  (if (<= (`/Game/Blueprint/Character_BP/MyCharacterBP.Lifes` _asmy_character_bp) 0)
    (set `/Game/Blueprint/Character_BP/MyCharacterBP.HP` 0.0 _asmy_character_bp)
    (`self.K2_DestroyActor` _asmy_character_bp)
    (else
      (`self.K2_SetActorLocation` _asmy_character_bp (`/Game/Blueprint/Character_BP/MyCharacterBP.SpawnPoint` _asmy_character_bp) false true)
      (set `/Game/Blueprint/Character_BP/MyCharacterBP.Lifes` (- (`/Game/Blueprint/Character_BP/MyCharacterBP.Lifes` _asmy_character_bp) 1) _asmy_character_bp)
      (set `/Game/Blueprint/Character_BP/MyCharacterBP.HP` 1.0 _asmy_character_bp))))

(fn `UserConstructionScript`)