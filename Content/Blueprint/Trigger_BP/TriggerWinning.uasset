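; TriggerWinning is a temporary last-player-standing win check for up to four local players, pending a better winning screen.
; Every Tick, a Sequence tests each player character for remaining Lifes, all three others at zero, and IsGameStarted.
; A match writes the win text to player 1's character, adds a Winning_Screen widget and sets WinningPlayer on KnNGameMode.
; Winners other than player 1 are also removed with their pawn; nothing latches the check.
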(event `self.ReceiveTick`
  (params (DeltaSeconds :type "Float (single-precision)"))
  ;[1 1 1] Überprüfen ob jemand gewonnen hat....ist nur vorrübergehend und wir noch in weiterentwicklung durch einen besseren Winningscreen ersetzt - Tim
  (`|ExecutionSequence`
    (:`then_0`
      (bind _asmy_character_bp (cast `/Game/Blueprint/Character_BP/MyCharacterBP` (`GameplayStatics.GetPlayerCharacter` 0)))
      (bind _lifes (`/Game/Blueprint/Character_BP/MyCharacterBP.Lifes` _asmy_character_bp))
      (bind _lifes_2 (`/Game/Blueprint/Character_BP/MyCharacterBP.Lifes` (stale _asmy_character_bp_2)))
      (bind _lifes_3 (`/Game/Blueprint/Character_BP/MyCharacterBP.Lifes` (stale _asmy_character_bp_3)))
      (bind _lifes_4 (`/Game/Blueprint/Character_BP/MyCharacterBP.Lifes` (stale _asmy_character_bp_4)))
      (if (and (> _lifes 0) (== _lifes_2 0) (== _lifes_3 0) (== _lifes_4 0) (`/Game/Blueprint/Character_BP/MyCharacterBP.IsGameStarted` _asmy_character_bp))
        (set `/Game/Blueprint/Character_BP/MyCharacterBP.Winning_String` "Player 1 Win" _asmy_character_bp)
        (bind _returnvalue (`|CreateWidget` "/Game/Blueprint/UI_Blueprints/Winning_Screen.Winning_Screen_C"))
        (`UserWidget.AddToViewport` _returnvalue 0)
        (bind _askn_ngame_mode (cast `/Game/Gamemodes/KnNGameMode` (`GameplayStatics.GetGameMode`)))
        (set `/Game/Gamemodes/KnNGameMode.WinningPlayer` 1 _askn_ngame_mode)))
    (:`then_1`
      (bind _asmy_character_bp_2 (cast `/Game/Blueprint/Character_BP/MyCharacterBP` (`GameplayStatics.GetPlayerCharacter` 1)))
      (if (and (> _lifes_2 0) (== _lifes 0) (== _lifes_3 0) (== _lifes_4 0) (`/Game/Blueprint/Character_BP/MyCharacterBP.IsGameStarted` _asmy_character_bp_2))
        (set `/Game/Blueprint/Character_BP/MyCharacterBP.Winning_String` "Player 2 Win" _asmy_character_bp)
        (bind _returnvalue_2 (`|CreateWidget` "/Game/Blueprint/UI_Blueprints/Winning_Screen.Winning_Screen_C"))
        (`UserWidget.AddToViewport` _returnvalue_2 0)
        (bind _askn_ngame_mode_2 (cast `/Game/Gamemodes/KnNGameMode` (`GameplayStatics.GetGameMode`)))
        (set `/Game/Gamemodes/KnNGameMode.WinningPlayer` 2 _askn_ngame_mode_2)
        (`GameplayStatics.RemovePlayer` (`GameplayStatics.GetPlayerController` 1) true)))
    (:`then_2`
      (bind _asmy_character_bp_3 (cast `/Game/Blueprint/Character_BP/MyCharacterBP` (`GameplayStatics.GetPlayerCharacter` 2)))
      (if (and (> _lifes_3 0) (== _lifes 0) (== _lifes_2 0) (== _lifes_4 0) (`/Game/Blueprint/Character_BP/MyCharacterBP.IsGameStarted` _asmy_character_bp_3))
        (set `/Game/Blueprint/Character_BP/MyCharacterBP.Winning_String` "Player 3 Win" _asmy_character_bp)
        (bind _returnvalue_3 (`|CreateWidget` "/Game/Blueprint/UI_Blueprints/Winning_Screen.Winning_Screen_C"))
        (`UserWidget.AddToViewport` _returnvalue_3 0)
        (bind _askn_ngame_mode_3 (cast `/Game/Gamemodes/KnNGameMode` (`GameplayStatics.GetGameMode`)))
        (set `/Game/Gamemodes/KnNGameMode.WinningPlayer` 3 _askn_ngame_mode_3)
        (`GameplayStatics.RemovePlayer` (`GameplayStatics.GetPlayerController` 2) true)))
    (:`then_3`
      (bind _asmy_character_bp_4 (cast `/Game/Blueprint/Character_BP/MyCharacterBP` (`GameplayStatics.GetPlayerCharacter` 3)))
      (if (and (> _lifes_4 0) (== _lifes 0) (== _lifes_2 0) (== _lifes_3 0) (`/Game/Blueprint/Character_BP/MyCharacterBP.IsGameStarted` _asmy_character_bp_4))
        (set `/Game/Blueprint/Character_BP/MyCharacterBP.Winning_String` "Player 4 Win" _asmy_character_bp)
        (bind _returnvalue_4 (`|CreateWidget` "/Game/Blueprint/UI_Blueprints/Winning_Screen.Winning_Screen_C"))
        (`UserWidget.AddToViewport` _returnvalue_4 0)
        (bind _askn_ngame_mode_4 (cast `/Game/Gamemodes/KnNGameMode` (`GameplayStatics.GetGameMode`)))
        (set `/Game/Gamemodes/KnNGameMode.WinningPlayer` 4 _askn_ngame_mode_4)
        (`GameplayStatics.RemovePlayer` (`GameplayStatics.GetPlayerController` 3) true)))))

(fn `UserConstructionScript`)