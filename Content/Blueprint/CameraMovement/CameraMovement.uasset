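; Shared Smash Bros-style camera actor for four players, noted by its author as an unfinished, poorly working attempt.
; BeginPlay makes it every player's view target and caches four MyCharacterBP actors.
; Each Tick finds the farthest-apart pair and interpolates the actor toward their midpoint.
; Clamped spring arm length derives from the interpolated position's distance to world origin, not the stored player separation, and sets the next interpolation speed.
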(event `self.ReceiveBeginPlay`
  ;[1 1 1] Kläglicher Versuch eine Smash Bros Cameraführung zu Programmieren...funktioniert also nicht wirklich gut...werde ich nach der Goldabgabe weiterprogrammieren aber bis zur Goldabgabe werde ich es nicht mehr schaffen - Tim
  (`PlayerController.SetViewTargetWithBlend` (`GameplayStatics.GetPlayerController` 0) self 0.0 "VTBlend_Linear" 0.0 false)
  (`PlayerController.SetViewTargetWithBlend` (`GameplayStatics.GetPlayerController` 1) self 0.0 "VTBlend_Linear" 0.0 false)
  (`PlayerController.SetViewTargetWithBlend` (`GameplayStatics.GetPlayerController` 2) self 0.0 "VTBlend_Linear" 0.0 false)
  (`PlayerController.SetViewTargetWithBlend` (`GameplayStatics.GetPlayerController` 3) self 0.0 "VTBlend_Linear" 0.0 false)
  (bind _outactors (`GameplayStatics.GetAllActorsOfClass` "/Game/Blueprint/Character_BP/MyCharacterBP.MyCharacterBP_C"))
  (for _index (range 4)
    (switch `int` _index
      (:`0`
        (bind _output (`|GetArrayItem` _outactors _index))
        (set `self.Character1` _output))
      (:`1`
        (set `self.Character2` _output))
      (:`2`
        (set `self.Character3` _output))
      (:`3`
        (set `self.Character4` _output)))))

(event `self.ReceiveTick`
  (params (DeltaSeconds :type "Float (single-precision)"))
  (bind _index (`self.Index`))
  (bind _returnvalue (`KismetMathLibrary.VInterpTo` (`self.Old Pos`) (`self.New Pos`) (`GameplayStatics.GetWorldDeltaSeconds`) (`self.Interp Speed`)))
  (bind (_indexofmaxvalue _maxvalue) (`KismetMathLibrary.MaxOfFloatArray` (`|MakeArray` (`KismetMathLibrary.Abs` (`KismetMathLibrary.VSize` (- (`self.K2_GetActorLocation` (`self.Character1`)) (`self.K2_GetActorLocation` (`self.Character2`))))) (`KismetMathLibrary.Abs` (`KismetMathLibrary.VSize` (- (`self.K2_GetActorLocation` (`self.Character1`)) (`self.K2_GetActorLocation` (`self.Character3`))))) (`KismetMathLibrary.Abs` (`KismetMathLibrary.VSize` (- (`self.K2_GetActorLocation` (`self.Character1`)) (`self.K2_GetActorLocation` (`self.Character4`))))) (`KismetMathLibrary.Abs` (`KismetMathLibrary.VSize` (- (`self.K2_GetActorLocation` (`self.Character2`)) (`self.K2_GetActorLocation` (`self.Character3`))))) (`KismetMathLibrary.Abs` (`KismetMathLibrary.VSize` (- (`self.K2_GetActorLocation` (`self.Character2`)) (`self.K2_GetActorLocation` (`self.Character4`))))) (`KismetMathLibrary.Abs` (`KismetMathLibrary.VSize` (- (`self.K2_GetActorLocation` (`self.Character3`)) (`self.K2_GetActorLocation` (`self.Character4`))))))))
  ;[1 1 1] Kläglicher Versuch eine Smash Bros Cameraführung zu Programmieren...funktioniert also nicht wirklich gut...werde ich nach der Goldabgabe weiterprogrammieren aber bis zur Goldabgabe werde ich es nicht mehr schaffen - Tim
  (set `self.Index` _indexofmaxvalue)
  (set `self.Distance` (`KismetMathLibrary.Conv_DoubleToVector` _maxvalue))
  (if (== _index 0)
    (`self.Func_P1_to_P2`)
    (bind _output_get (set `self.Focus` _returnvalue :!label _label))
    (`self.K2_SetActorLocation` _output_get)
    (set `self.Old Pos` (`self.K2_GetActorLocation`))
    (bind _output_get_2 (set `SpringArmComponent.TargetArmLength` (`KismetMathLibrary.FClamp` (* (`KismetMathLibrary.VSize` _returnvalue) 1.2) 600.0 2000.0) (`self.SpringArm`)))
    (set `self.Interp Speed` (/ _output_get_2 600.0))
    (elif (== _index 1)
      (`self.Func_P1_to_P3`)
      (goto _label)
      (elif (== _index 2)
        (`self.Func_P1_to_P4`)
        (goto _label)
        (elif (== _index 3)
          (`self.Func_P2_to_P3`)
          (goto _label)
          (elif (== _index 4)
            (`self.Func_P2_to_P4`)
            (goto _label)
            (elif (== _index 5)
              (`self.Func_P3_to_P4`)
              (goto _label))))))))

(fn `Func_P1_to_P2`
  (set `self.New Pos` (/ (+ (`self.K2_GetActorLocation` (`self.Character1`)) (`self.K2_GetActorLocation` (`self.Character2`))) 2.0)))

(fn `Func_P1_to_P3`
  (set `self.New Pos` (/ (+ (`self.K2_GetActorLocation` (`self.Character1`)) (`self.K2_GetActorLocation` (`self.Character3`))) 2.0)))

(fn `Func_P1_to_P4`
  (set `self.New Pos` (/ (+ (`self.K2_GetActorLocation` (`self.Character1`)) (`self.K2_GetActorLocation` (`self.Character4`))) 2.0)))

(fn `Func_P2_to_P3`
  (set `self.New Pos` (/ (+ (`self.K2_GetActorLocation` (`self.Character2`)) (`self.K2_GetActorLocation` (`self.Character3`))) 2.0)))

(fn `Func_P2_to_P4`
  (set `self.New Pos` (/ (+ (`self.K2_GetActorLocation` (`self.Character2`)) (`self.K2_GetActorLocation` (`self.Character4`))) 2.0)))

(fn `Func_P3_to_P4`
  (set `self.New Pos` (/ (+ (`self.K2_GetActorLocation` (`self.Character3`)) (`self.K2_GetActorLocation` (`self.Character4`))) 2.0)))

(fn `UserConstructionScript`)