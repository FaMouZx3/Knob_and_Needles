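; Main menu pawn that relays a player's UI input to the active menu widget and shows cosmetic clothing.
; Fire and directional presses read the game mode's ActiveWidgetId and call the matching character selection, map selection or main menu widget, passing PlayerID only to character selection.
; On BeginPlay, SetClothes sets socket meshes from Head, Face and Body indices.
; FStart yaws the pawn toward the camera, but its event graph call is disconnected.
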(event `self.ReceiveBeginPlay`
  (`self.SetClothes`))

(event `self.ReceiveActorBeginOverlap`
  (params (OtherActor :type "Actor Object Reference")))

(event `self.ReceiveTick`
  (params (DeltaSeconds :type "Float (single-precision)")))

(event `InputAction|UI Fire`
  (params (Key :type "Key Structure" :default "AnyKey"))
  (:`Pressed`
    (bind _asmain_menu_game_mode_widget (cast `/Game/Blueprint/MainMenu/MainMenuGameModeWidget` (`GameplayStatics.GetGameMode`)))
    (switch `int` (`/Game/Blueprint/MainMenu/MainMenuGameModeWidget.ActiveWidgetId` _asmain_menu_game_mode_widget)
      (:`Default`
        (bind _activewidget (`/Game/Blueprint/MainMenu/MainMenuGameModeWidget.ActiveWidget` _asmain_menu_game_mode_widget))
        (bind _ascharacter_selection (cast `/Game/Blueprint/MainMenu/CharacterSelection` _activewidget :!label _label))
        (`/Game/Blueprint/MainMenu/CharacterSelection.F Fire` _ascharacter_selection (`self.Player ID`)))
      (:`0`
        (goto _label))
      (:`1`
        (bind _asmap_selection_widget (cast `/Game/Blueprint/MainMenu/MapSelectionWidget` _activewidget))
        (`/Game/Blueprint/MainMenu/MapSelectionWidget.F Fire` _asmap_selection_widget))
      (:`2`
        (bind _asmain_menu_widget (cast `/Game/Blueprint/MainMenu/MainMenuWidget` _activewidget))
        (`/Game/Blueprint/MainMenu/MainMenuWidget.F Fire` _asmain_menu_widget)))))

(event `InputAction|UI Up`
  (params (Key :type "Key Structure" :default "AnyKey"))
  (:`Pressed`
    (bind _asmain_menu_game_mode_widget (cast `/Game/Blueprint/MainMenu/MainMenuGameModeWidget` (`GameplayStatics.GetGameMode`)))
    (switch `int` (`/Game/Blueprint/MainMenu/MainMenuGameModeWidget.ActiveWidgetId` _asmain_menu_game_mode_widget)
      (:`Default`
        (bind _activewidget (`/Game/Blueprint/MainMenu/MainMenuGameModeWidget.ActiveWidget` _asmain_menu_game_mode_widget))
        (bind _ascharacter_selection (cast `/Game/Blueprint/MainMenu/CharacterSelection` _activewidget :!label _label_2))
        (`/Game/Blueprint/MainMenu/CharacterSelection.F Input Up` _ascharacter_selection (`self.Player ID`)))
      (:`0`
        (goto _label_2))
      (:`1`
        (bind _asmap_selection_widget (cast `/Game/Blueprint/MainMenu/MapSelectionWidget` _activewidget))
        (`/Game/Blueprint/MainMenu/MapSelectionWidget.F Input Up` _asmap_selection_widget))
      (:`2`
        (bind _asmain_menu_widget (cast `/Game/Blueprint/MainMenu/MainMenuWidget` _activewidget))
        (`/Game/Blueprint/MainMenu/MainMenuWidget.F Input Up` _asmain_menu_widget)))))

(event `InputAction|UI Down`
  (params (Key :type "Key Structure" :default "AnyKey"))
  (:`Pressed`
    (bind _asmain_menu_game_mode_widget (cast `/Game/Blueprint/MainMenu/MainMenuGameModeWidget` (`GameplayStatics.GetGameMode`)))
    (switch `int` (`/Game/Blueprint/MainMenu/MainMenuGameModeWidget.ActiveWidgetId` _asmain_menu_game_mode_widget)
      (:`Default`
        (bind _activewidget (`/Game/Blueprint/MainMenu/MainMenuGameModeWidget.ActiveWidget` _asmain_menu_game_mode_widget))
        (bind _ascharacter_selection (cast `/Game/Blueprint/MainMenu/CharacterSelection` _activewidget :!label _label_3))
        (`/Game/Blueprint/MainMenu/CharacterSelection.F Input Down` _ascharacter_selection (`self.Player ID`)))
      (:`0`
        (goto _label_3))
      (:`1`
        (bind _asmap_selection_widget (cast `/Game/Blueprint/MainMenu/MapSelectionWidget` _activewidget))
        (`/Game/Blueprint/MainMenu/MapSelectionWidget.F Input Down` _asmap_selection_widget))
      (:`2`
        (bind _asmain_menu_widget (cast `/Game/Blueprint/MainMenu/MainMenuWidget` _activewidget))
        (`/Game/Blueprint/MainMenu/MainMenuWidget.F Input Down` _asmain_menu_widget)))))

(event `InputAction|UI Right`
  (params (Key :type "Key Structure" :default "AnyKey"))
  (:`Pressed`
    (bind _asmain_menu_game_mode_widget (cast `/Game/Blueprint/MainMenu/MainMenuGameModeWidget` (`GameplayStatics.GetGameMode`)))
    (switch `int` (`/Game/Blueprint/MainMenu/MainMenuGameModeWidget.ActiveWidgetId` _asmain_menu_game_mode_widget)
      (:`Default`
        (bind _activewidget (`/Game/Blueprint/MainMenu/MainMenuGameModeWidget.ActiveWidget` _asmain_menu_game_mode_widget))
        (bind _ascharacter_selection (cast `/Game/Blueprint/MainMenu/CharacterSelection` _activewidget :!label _label_4))
        (`/Game/Blueprint/MainMenu/CharacterSelection.F Input Right` _ascharacter_selection (`self.Player ID`)))
      (:`0`
        (goto _label_4))
      (:`1`
        (bind _asmap_selection_widget (cast `/Game/Blueprint/MainMenu/MapSelectionWidget` _activewidget))
        (`/Game/Blueprint/MainMenu/MapSelectionWidget.F Input Right` _asmap_selection_widget))
      (:`2`
        (bind _asmain_menu_widget (cast `/Game/Blueprint/MainMenu/MainMenuWidget` _activewidget))
        (`/Game/Blueprint/MainMenu/MainMenuWidget.F Input Right` _asmain_menu_widget)))))

(event `InputAction|UI Left`
  (params (Key :type "Key Structure" :default "AnyKey"))
  (:`Pressed`
    (bind _asmain_menu_game_mode_widget (cast `/Game/Blueprint/MainMenu/MainMenuGameModeWidget` (`GameplayStatics.GetGameMode`)))
    (switch `int` (`/Game/Blueprint/MainMenu/MainMenuGameModeWidget.ActiveWidgetId` _asmain_menu_game_mode_widget)
      (:`Default`
        (bind _activewidget (`/Game/Blueprint/MainMenu/MainMenuGameModeWidget.ActiveWidget` _asmain_menu_game_mode_widget))
        (bind _ascharacter_selection (cast `/Game/Blueprint/MainMenu/CharacterSelection` _activewidget :!label _label_5))
        (`/Game/Blueprint/MainMenu/CharacterSelection.F Input Left` _ascharacter_selection (`self.Player ID`)))
      (:`0`
        (goto _label_5))
      (:`1`
        (bind _asmap_selection_widget (cast `/Game/Blueprint/MainMenu/MapSelectionWidget` _activewidget))
        (`/Game/Blueprint/MainMenu/MapSelectionWidget.F Input Left` _asmap_selection_widget))
      (:`2`
        (bind _asmain_menu_widget (cast `/Game/Blueprint/MainMenu/MainMenuWidget` _activewidget))
        (`/Game/Blueprint/MainMenu/MainMenuWidget.F Input Left` _asmain_menu_widget)))))

(fn `F Start`
  (`self.K2_SetActorRotation` (`KismetMathLibrary.MakeRotator` 0.0 0.0 (+ (.yaw (`KismetMathLibrary.FindLookAtRotation` (`self.K2_GetActorLocation`) (`self.K2_GetActorLocation` (`GameplayStatics.GetPlayerCameraManager` 0)))) -90.0)) true))

(fn `GetActiveWidget`
  (returns (Widget :type "Widget Class Reference"))
  (bind _asmain_menu_game_mode_widget (cast `/Game/Blueprint/MainMenu/MainMenuGameModeWidget` (`GameplayStatics.GetGameMode`)))
  (bind _ascharacter_selection (cast `/Game/Blueprint/MainMenu/CharacterSelection` (`/Game/Blueprint/MainMenu/MainMenuGameModeWidget.ActiveWidget` _asmain_menu_game_mode_widget)))
  (return (`GameplayStatics.GetObjectClass` _ascharacter_selection)))

(fn `SetClothes`
  (switch `int` (`self.Head`)
    (:`0`
      (set `self.MeshTmp` null))
    (:`1`
      (bind _output_get (set `self.MeshTmp` "/Game/Meshes/Costumes/Head/Cu_Mage_Hat_01_Hat002.Cu_Mage_Hat_01_Hat002"))))
  (`StaticMeshComponent.SetStaticMesh` (`self. HeadSocket`) _output_get)
  (switch `int` (`self.Face`)
    (:`0`
      (bind _output_get_2 (set `self.MeshTmp` null)))
    (:`1`
      (set `self.MeshTmp` "/Game/Meshes/Costumes/Face/Cu_Nerd_glasses_01.Cu_Nerd_glasses_01")))
  (`StaticMeshComponent.SetStaticMesh` (`self.FaceSocket`) _output_get_2)
  (switch `int` (`self.Body`)
    (:`0`
      (set `self.MeshTmp` null)
      (`StaticMeshComponent.SetStaticMesh` (`self.BodySocket`) null))))

(fn `UserConstructionScript`)