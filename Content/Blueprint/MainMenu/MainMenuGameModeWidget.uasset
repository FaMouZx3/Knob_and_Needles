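; Main menu game mode that swaps between main menu, map selection, character selection and credits screens, opening the main menu on BeginPlay.
; Each load function clears all widgets, shows its own and records the active widget and ID; map selection and credits share an ID.
; Character selection also creates three extra local players, places all four pawns at a Helper actor's spawn points and initializes the new UIInputPawns with player IDs.
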(event `self.ReceiveBeginPlay`
  (`self.LoadMainMenu`))

(event `self.ReceiveTick`
  (params (DeltaSeconds :type "Float (single-precision)")))

(event `self.ReceiveEndPlay`
  (params (EndPlayReason :type "EEndPlayReason Enum" :default "Destroyed"))
  (cast `GameInstance` (`GameplayStatics.GetGameInstance`)))

(fn `LoadCharacter Selection`
  (bind _outactors (`GameplayStatics.GetAllActorsOfClass` "/Game/Blueprint/MainMenu/helper.helper_C"))
  (set `self.Spawns` (`/Game/Blueprint/MainMenu/helper.spwnpts` (`|GetArrayItem` _outactors)))
  (for _index (range 1 4)
    (bind _returnvalue (`GameplayStatics.CreatePlayer` -1))
    (`GameplayStatics.GetPlayerControllerID` _returnvalue)
    (for (_array_element _array_index) (`self.Spawns`)
      (if (== _index _array_index)
        (bind _returnvalue_2 (`Controller.K2_GetPawn` _returnvalue))
        (`self.K2_SetActorLocation` _returnvalue_2 (`self.K2_GetActorLocation` _array_element) false true)
        (bind _asuiinput_pawn (cast `/Game/Blueprint/MainMenu/UIInputPawn` _returnvalue_2))
        (set `/Game/Blueprint/MainMenu/UIInputPawn.Player ID` _index _asuiinput_pawn)
        (`/Game/Blueprint/MainMenu/UIInputPawn.F Start` _asuiinput_pawn))))
  (`self.K2_SetActorLocation` (`Controller.K2_GetPawn` (`GameplayStatics.GetPlayerController` 0)) (`self.K2_GetActorLocation` (`|GetArrayItem` (`self.Spawns`))) false false)
  (`WidgetLayoutLibrary.RemoveAllWidgets`)
  (bind _returnvalue_3 (`|CreateWidget` "/Game/Blueprint/MainMenu/CharacterSelection.CharacterSelection_C" (`GameplayStatics.GetPlayerController` 0)))
  (set `self.ActiveWidget` _returnvalue_3)
  (`UserWidget.AddToViewport` _returnvalue_3 0)
  (set `self.ActiveWidgetId` 0))

(fn `LoadCredits`
  (`WidgetLayoutLibrary.RemoveAllWidgets`)
  (bind _returnvalue (`|CreateWidget` "/Game/Blueprint/MainMenu/CreditsWidget.CreditsWidget_C" (`GameplayStatics.GetPlayerController` 0)))
  (set `self.ActiveWidget` _returnvalue)
  (`UserWidget.AddToViewport` _returnvalue 0)
  (set `self.ActiveWidgetId` 1))

(fn `LoadMainMenu`
  (`WidgetLayoutLibrary.RemoveAllWidgets`)
  (bind _returnvalue (`|CreateWidget` "/Game/Blueprint/MainMenu/MainMenuWidget.MainMenuWidget_C" (`GameplayStatics.GetPlayerController` 0)))
  (set `self.ActiveWidget` _returnvalue)
  (`UserWidget.AddToViewport` _returnvalue 0)
  (set `self.ActiveWidgetId` 2))

(fn `LoadMapSelection`
  (`WidgetLayoutLibrary.RemoveAllWidgets`)
  (bind _returnvalue (`|CreateWidget` "/Game/Blueprint/MainMenu/MapSelectionWidget.MapSelectionWidget_C" (`GameplayStatics.GetPlayerController` 0)))
  (set `self.ActiveWidget` _returnvalue)
  (`UserWidget.AddToViewport` _returnvalue 0)
  (set `self.ActiveWidgetId` 1))

(fn `UserConstructionScript`)