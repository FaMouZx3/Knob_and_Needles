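; Cel-shading lighting helper that copies scene light data into parameters on an array of materials.
; UpdateLights writes colour, position, attenuation and intensity for up to two point lights, plus the first directional light's colour, direction and intensity.
; GatherPointLights orders all point lights by distance to a location only roughly, front-inserting any closer than a listed one, so the first two may not be nearest.
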(fn `GatherPointLights`
  (params (Location :type "Vector Structure"))
  (returns (Lights :type "Array of /Game/Shaders/CelLightingModel/Blueprints/LightAndDistance Structure"))
  (locals (LocalLights :type "Array of /Game/Shaders/CelLightingModel/Blueprints/LightAndDistance Structure") (Found :type Boolean :default false))
  (`KismetArrayLibrary.Array_Clear` (`local.LocalLights`))
  (bind _outactors (`GameplayStatics.GetAllActorsOfClass` null "/Script/Engine.PointLight"))
  (for _array_element _outactors
    (set `local.Found` false)
    (if (== (`KismetArrayLibrary.Array_Length` (`local.LocalLights`)) 0)
      (bind _lightanddistance (make `/Game/Shaders/CelLightingModel/Blueprints/LightAndDistance` (`PointLight.PointLightComponent` _array_element) (`KismetMathLibrary.VSize` (- Location (`Actor.K2_GetActorLocation` _array_element)))))
      (`KismetArrayLibrary.Array_Add` (`local.LocalLights`) _lightanddistance)
      (else
        (for _array_element_2 (`local.LocalLights`)
          (if (> (`.Distance_5_72C424EB4BAF743ECAEC83AF0696112C` (break `/Game/Shaders/CelLightingModel/Blueprints/LightAndDistance` _array_element_2)) (`.Distance_5_72C424EB4BAF743ECAEC83AF0696112C` (break `/Game/Shaders/CelLightingModel/Blueprints/LightAndDistance` _lightanddistance)))
            (`KismetArrayLibrary.Array_Insert` (`local.LocalLights`) _lightanddistance)
            (set `local.Found` true)
            (break)))
        (if (not (`local.Found`))
          (`KismetArrayLibrary.Array_Add` (`local.LocalLights`) _lightanddistance)))))
  (return (`local.LocalLights`)))

(fn `UpdateLights`
  (params (Material :type "Array of MaterialInstanceDynamic Object Reference") (Location :type "Vector Structure"))
  (for _array_element Material
    (`|ExecutionSequence`
      (:`then_0`
        (bind _lights (`self.GatherPointLights` Location))
        (`|ExecutionSequence`
          (:`then_0`
            (bind _light (break `/Game/Shaders/CelLightingModel/Blueprints/LightAndDistance` (`KismetArrayLibrary.Array_Get` _lights)))
            (`MaterialInstanceDynamic.SetVectorParameterValue` _array_element "LightColour1" (`LightComponentBase.GetLightColor` _light))
            (`MaterialInstanceDynamic.SetVectorParameterValue` _array_element "LightPosition1" (`KismetMathLibrary.Conv_VectorToLinearColor` (`SceneComponent.K2_GetComponentLocation` _light)))
            (`MaterialInstanceDynamic.SetScalarParameterValue` _array_element "LightAttenuation1" (`PointLightComponent.AttenuationRadius` _light))
            (`MaterialInstanceDynamic.SetScalarParameterValue` _array_element "LightIntensity1" (`LightComponentBase.Intensity` _light)))
          (:`then_1`
            (if (> (`KismetArrayLibrary.Array_Length` _lights) 1)
              (bind _light_2 (break `/Game/Shaders/CelLightingModel/Blueprints/LightAndDistance` (`KismetArrayLibrary.Array_Get` _lights 1)))
              (`MaterialInstanceDynamic.SetVectorParameterValue` _array_element "LightColour2" (`LightComponentBase.GetLightColor` _light_2))
              (`MaterialInstanceDynamic.SetVectorParameterValue` _array_element "LightPosition2" (`KismetMathLibrary.Conv_VectorToLinearColor` (`SceneComponent.K2_GetComponentLocation` _light_2)))
              (`MaterialInstanceDynamic.SetScalarParameterValue` _array_element "LightAttenuation2" (`PointLightComponent.AttenuationRadius` _light_2))
              (`MaterialInstanceDynamic.SetScalarParameterValue` _array_element "LightIntensity2" (`LightComponentBase.Intensity` _light_2))))))
      (:`then_1`
        (bind _outactors (`GameplayStatics.GetAllActorsOfClass` null "/Script/Engine.DirectionalLight"))
        (bind _lightcomponent (`Light.LightComponent` (`KismetArrayLibrary.Array_Get` _outactors)))
        (`MaterialInstanceDynamic.SetVectorParameterValue` _array_element "SunColour" (`LightComponentBase.GetLightColor` _lightcomponent))
        (`MaterialInstanceDynamic.SetVectorParameterValue` _array_element "SunDirection" (`KismetMathLibrary.Conv_VectorToLinearColor` (`KismetMathLibrary.BreakRotIntoAxes` (`SceneComponent.K2_GetComponentRotation` _lightcomponent))))
        (`MaterialInstanceDynamic.SetScalarParameterValue` _array_element "SunIntensity" (`LightComponentBase.Intensity` _lightcomponent))))))