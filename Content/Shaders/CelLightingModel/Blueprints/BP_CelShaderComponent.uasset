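; Actor component that drives cel shading on its owning Skeletal Mesh or Static Mesh actor.
; On BeginPlay it replaces the mesh's materials with dynamic instances, stores them and caches the mesh component; the static mesh path always writes to element 0.
; Every Tick it passes those materials and the mesh's world location to UpdateLights to refresh the lighting.
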(event `self.ReceiveBeginPlay`
  (bind _returnvalue (`self.GetOwner`))
  (bind _materials (`self.Materials`))
  ;[0 0 0] Find and configure components to cel shade
  (`|ExecutionSequence`
    (:`then_0`
      (bind _asskeletal_mesh_actor (cast `SkeletalMeshActor` _returnvalue)) ; Find materials in skeletal meshes
      (bind _skeletalmeshcomponent (`SkeletalMeshActor.SkeletalMeshComponent` _asskeletal_mesh_actor))
      (set `self.ReferencedComponent` _skeletalmeshcomponent)
      (for (_array_element _array_index) (`MeshComponent.GetMaterials` _skeletalmeshcomponent)
        (bind _returnvalue_2 (`PrimitiveComponent.CreateDynamicMaterialInstance` _skeletalmeshcomponent _array_index _array_element))
        (`KismetArrayLibrary.Array_Add` _materials _returnvalue_2)
        (`/Game/Shaders/CelLightingModel/Blueprints/BPF_CelLighting.UpdateLights` _materials (`SceneComponent.K2_GetComponentLocation` _skeletalmeshcomponent))))
    (:`then_1`
      (bind _asstatic_mesh_actor (cast `StaticMeshActor` _returnvalue)) ; Find materials in static meshes
      (bind _staticmeshcomponent (`StaticMeshActor.StaticMeshComponent` _asstatic_mesh_actor))
      (set `self.ReferencedComponent` _staticmeshcomponent)
      (for _array_element_2 (`MeshComponent.GetMaterials` _staticmeshcomponent)
        (bind _returnvalue_3 (`PrimitiveComponent.CreateDynamicMaterialInstance` _staticmeshcomponent 0 _array_element_2))
        (`KismetArrayLibrary.Array_Add` _materials _returnvalue_3)
        (`/Game/Shaders/CelLightingModel/Blueprints/BPF_CelLighting.UpdateLights` _materials (`SceneComponent.K2_GetComponentLocation` _staticmeshcomponent))))))

(event `self.ReceiveTick`
  (params (DeltaSeconds :type "Float (single-precision)"))
  (bind _referencedcomponent (`self.ReferencedComponent`))
  (bind _materials (`self.Materials`))
  ;[0 0 0] Update lighting
  (`|ExecutionSequence`
    (:`then_0`
      (bind _asskeletal_mesh_component (cast `SkeletalMeshComponent` _referencedcomponent))
      (`/Game/Shaders/CelLightingModel/Blueprints/BPF_CelLighting.UpdateLights` _materials (`SceneComponent.K2_GetComponentLocation` _asskeletal_mesh_component)))
    (:`then_1`
      (bind _asstatic_mesh_component (cast `StaticMeshComponent` _referencedcomponent))
      (`/Game/Shaders/CelLightingModel/Blueprints/BPF_CelLighting.UpdateLights` _materials (`SceneComponent.K2_GetComponentLocation` _asstatic_mesh_component)))))