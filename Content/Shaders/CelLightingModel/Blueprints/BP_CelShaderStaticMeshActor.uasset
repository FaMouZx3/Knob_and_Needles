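; A static mesh actor Blueprint for a cel lighting model that keeps its materials updated with lighting for its position.
; The construction script creates a dynamic material instance for each mesh material slot, stores it in an array and passes that array and the actor location to UpdateLights.
; On Tick, it calls UpdateLights again only when the actor has moved beyond a tiny tolerance, then caches the new location.
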(event `self.ReceiveTick`
  (params (DeltaSeconds :type "Float (single-precision)"))
  (bind _returnvalue (`self.K2_GetActorLocation`))
  (if (not (== _returnvalue (`self.OldLocation`)))
    (`/Game/Shaders/CelLightingModel/Blueprints/BPF_CelLighting.UpdateLights` (`self.Material`) _returnvalue)
    (set `self.OldLocation` _returnvalue)))

(fn `UserConstructionScript`
  (bind _staticmeshcomponent (`self.StaticMeshComponent`))
  (bind _material (`self.Material`))
  (for (_array_element _array_index) (`MeshComponent.GetMaterials` _staticmeshcomponent)
    (bind _returnvalue (`PrimitiveComponent.CreateDynamicMaterialInstance` _staticmeshcomponent _array_index _array_element))
    (`KismetArrayLibrary.Array_Add` _material _returnvalue)
    (`/Game/Shaders/CelLightingModel/Blueprints/BPF_CelLighting.UpdateLights` _material (`self.K2_GetActorLocation`))))